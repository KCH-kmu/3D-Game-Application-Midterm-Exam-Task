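; BP_Enemy is an enemy that pursues the player character and can be killed by damage.
; From BeginPlay it runs AIMoveTo toward the player, restarting on each success, with no handling for a failed move.
; AnyDamage subtracts from a truncated Health value and destroys the actor at zero or below.
; Logic to spawn and socket-attach a weapon exists but is disconnected, so it never runs.
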(event Custom|Chase%20Player
  (AI|AIMoveTo self "0, 0, 0" (Game|GetPlayerCharacter 0) 5.0 false
    (:OnSuccess
      (CallFunction|ChasePlayer))))

(event EventBeginPlay
  (CallFunction|ChasePlayer))

(event Collision|EventActorBeginOverlap
  (params (OtherActor :type Actor%20Object%20Reference)))

(event EventTick
  (params (DeltaSeconds :type Float%20%28single-precision%29)))

(event Game|Damage|EventAnyDamage
  (params (Damage :type Float%20%28single-precision%29) (DamageType :type Damage%20Type%20Object%20Reference) (InstigatedBy :type Controller%20Object%20Reference) (DamageCauser :type Actor%20Object%20Reference))
  (Variables|Default|SetHealth (Math|Float|Truncate (- (Variables|Default|GetHealth) Damage)))
  (if (<= (Variables|Default|GetHealth) 0)
    (Actor|DestroyActor)))

(fn ConstructionScript)